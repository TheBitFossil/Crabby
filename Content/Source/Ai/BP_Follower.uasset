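; BP_Follower is a pawn that follows the player once the player has overlapped its Sphere1 component.
; The overlap stores the BP_Player reference, which is never cleared, so following continues after the player leaves the sphere.
; A looping 0.1-second timer, rather than Tick, feeds a scaled, normalized direction toward the player's current location into FloatingPawnMovement.
; Debug prints show the detected player, input vector and timer ticks.
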(event `self.ReceiveBeginPlay`
  (add `PrimitiveComponent.OnComponentBeginOverlap` (`self.Sphere1`) (delegate `CustomEvent_1`))
  (if (`KismetSystemLibrary.IsValid` (`self.GetMovementComponent`))
    (bind _returnvalue (`KismetSystemLibrary.K2_SetTimerDelegate` (delegate `CustomEvent`) 0.1 true true))
    (set `self.NewVar` _returnvalue)))

(event `CustomEvent_1`
  (params (OverlappedComponent :type "PrimitiveComponent Object Reference") (OtherActor :type "Actor Object Reference") (OtherComp :type "PrimitiveComponent Object Reference") (OtherBodyIndex :type Integer) (bFromSweep :type Boolean) (SweepResult :type "HitResult Structure (by ref)"))
  (bind _asbp_player (cast `/Game/Source/Player/BP_Player` OtherActor))
  (bind _output_get (set `self.As BP Player` _asbp_player))
  (set `self.PlayerLoc` (`self.K2_GetActorLocation` _output_get))
  (`KismetSystemLibrary.PrintString` (`KismetSystemLibrary.GetDisplayName` _output_get) true true (struct :`R` 0.714048 :`G` 0.006859 :`B` 1.0 :`A` 1.0)))

(event `CustomEvent`
  (bind _as_bp_player (`self.As BP Player`))
  (`/Engine/EditorBlueprintResources/StandardMacros.IsValid` _as_bp_player
    (:`Is Valid`
      (`PawnMovementComponent.AddInputVector` (`self.FloatingPawnMovement`) (* (`self.NewVar_0`) (`KismetMathLibrary.Normal` (- (`self.K2_GetActorLocation` _as_bp_player) (`self.K2_GetActorLocation`)))) true)
      (`KismetSystemLibrary.PrintString` (`KismetStringLibrary.Conv_VectorToString` (`PawnMovementComponent.GetLastInputVector` (`self.FloatingPawnMovement`))))
      (`KismetSystemLibrary.PrintString` "TImer TIck"))))

(fn `UserConstructionScript`)